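; BP_JsonWeather fetches live weather for a fixed city from the AMap REST API and passes it to the level.
; BeginPlay fires a single VaRest GET; the callback prints the first "lives" entry's weather text.
; WeatherIndex maps the Chinese text to an enum by exact match, then by cloud/rain/snow character at index 1, defaulting to overcast.
; The result goes to every BPI_Weather actor via SetweatherIdMessage.
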(event Custom|Callback
  (params (Request :type Va%20Rest%20Request%20JSON%20Object%20Reference))
  (bind _returnvalue (Class|VaRestRequestJSON|GetResponseObject Request))
  ;[1 1 1] 填写解析字段
  (Utilities|IsValid _returnvalue
    (:Is%20Valid
      (bind _returnvalue_2 (Class|VaRestJsonValue|AsObject (Utilities|Array|Get(acopy) (Class|VaRestJsonObject|GetArrayField _returnvalue "lives"))))
      (Development|PrintString (Class|VaRestJsonObject|GetStringField _returnvalue_2 "weather") true true "(R=0.000000,G=0.660000,B=1.000000,A=1.000000)" 1e+01)
      (bind _newparam1 (CallFunction|WeatherIndex (Class|VaRestJsonObject|GetStringField _returnvalue_2 "weather")))
      (bind _outactors (Actor|GetAllActorswithInterface "/Game/Blueprints/BPI_Weather.BPI_Weather_C"))
      (for _array_element _outactors
        (Class|BPIWeather|SetweatherId(Message) _array_element _newparam1)))))

(event Custom|SetWeather
  (params (NewParam :type String)))

(event EventBeginPlay
  (bind _returnvalue (|VaRestSubsystem))
  (Class|VaRestSubsystem|ConstructVaRestJsonObject _returnvalue)
  ;[1 1 1] url
  (Class|VaRestSubsystem|CallURL _returnvalue "https://restapi.amap.com/v3/weather/weatherInfo?city=310101&key=1082e9c4130f16162ebf6109285f7d7d" "GET" "x_www_form_urlencoded_url" 0 (delegate Custom|Callback)))

(event EventTick
  (params (DeltaSeconds :type Float%20%28single-precision%29)))

(fn ConstructionScript)

(fn WeatherIndex
  (params (NewParam :type String))
  (switch string NewParam
    (:Default
      (if (== (Utilities|String|FindSubstring NewParam "云") 1)
        (return "NewEnumerator2")
        (elif (== (Utilities|String|FindSubstring NewParam "雨") 1)
          (return "NewEnumerator6")
          (elif (== (Utilities|String|FindSubstring NewParam "雪") 1)
            (return "NewEnumerator8")
            (else
              (return "NewEnumerator11"))))))
    (:晴
      (return "NewEnumerator0"))
    (:多云
      (return "NewEnumerator2"))
    (:雨
      (return "NewEnumerator6"))
    (:阴
      (return "NewEnumerator11"))))